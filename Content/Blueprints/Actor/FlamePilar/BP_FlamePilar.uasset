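; Flame pillar actor that animates the intensity of its fire light to create a varying flicker.
; On BeginPlay it randomly picks one of two intensity timelines and picks again each time one finishes, forming an endless, non-repeating-looking loop.
; Each timeline update multiplies the curve value by a base intensity and applies it to the light.
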(event Custom|StartTimelineA
  (bind _pointlightintensitya (Timeline|FlameIntensityA PlayFromStart)
    (:Update
      (CallFunction|ScaleFlameIntensity _pointlightintensitya))
    (:Finished
      (CallFunction|ChooseTimeline))))

(event Custom|StartTimelineB
  (bind _pointlineintensityb (Timeline|FlameIntensityB PlayFromStart)
    (:Update
      (CallFunction|ScaleFlameIntensity _pointlineintensityb))
    (:Finished
      (CallFunction|ChooseTimeline))))

(event Custom|ChooseTimeline
  (if (Math|Random|RandomBool)
    (CallFunction|StartTimelineA)
    (else
      (CallFunction|StartTimelineB))))

(event EventBeginPlay
  (CallFunction|ChooseTimeline))

(fn ConstructionScript)

(fn ScaleFlameIntensity
  (params (Intensity :type Float%20%28double-precision%29))
  (Rendering|Components|Light|SetIntensity (Variables|Default|GetFIreLight) (* Intensity (Variables|Default|GetBaseIntensity))))