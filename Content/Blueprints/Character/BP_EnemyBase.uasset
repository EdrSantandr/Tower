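; BP_EnemyBase is a base enemy Blueprint that handles spawn and dissolve visuals plus motion-warp facing.
; On BeginPlay, a timeline scales the mesh uniformly while cumulatively adding yaw, then restores the initial rotation.
; Separate timelines drive the "Dissolve" parameter on dynamic materials passed to the mesh and weapon dissolve events.
; UpdateFacingTarget feeds a location into the "FacingTarget" motion warp target for smoother turning.
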(event EventBeginPlay
  (bind _mesh (Variables|Character|GetMesh))
  (bind _relativerotation (Variables|/Script/Engine.SceneComponent|GetRelativeRotation _mesh))
  (Variables|Default|SetInitialRotation (Variables|/Script/Engine.SceneComponent|GetRelativeRotation (Variables|Character|GetMesh)))
  (bind (_direction _scaletrack _rotationztrack) (Timeline|SpawnTimeline Play)
    (:Update
      (Transformation|SetRelativeScale3D _mesh (Math|Vector|MakeVector _scaletrack _scaletrack _scaletrack))
      (Transformation|SetRelativeRotation _mesh (Math|Rotator|MakeRotator (.roll _relativerotation) (.pitch _relativerotation) (+ _rotationztrack (.yaw _relativerotation))) false false))
    (:Finished
      (Transformation|SetRelativeRotation _mesh (Variables|Default|GetInitialRotation) false false))))

(event EventUpdateFacingTarget
  (params (Target :type Vector%20%28by%20ref%29 :default "0, 0, 0"))
  ;[1 1 1] We should update the target so the rotation can be more smoothly
  (Class|MotionWarpingComponent|AddorUpdateWarpTargetfromLocation (Variables|Default|GetMotionWarping) "FacingTarget" Target))

(event EventStartMeshDissolveTimeline
  (params (DynamicMaterial :type Material%20Instance%20Dynamic%20Object%20Reference))
  (bind _dissolvetrack (Timeline|DissolveMeshTimeline Play)
    (:Update
      (Rendering|Material|SetScalarParameterValue DynamicMaterial "Dissolve" _dissolvetrack :!class /Script/Engine.MaterialInstanceDynamic))))

(event EventStartWeaponDissolveTimeline
  (params (DynamicMaterial :type Material%20Instance%20Dynamic%20Object%20Reference))
  (bind _dissolvetrack (Timeline|DissolveWeaponTimeline Play)
    (:Update
      (Rendering|Material|SetScalarParameterValue DynamicMaterial "Dissolve" _dissolvetrack :!class /Script/Engine.MaterialInstanceDynamic))))

(fn ConstructionScript)